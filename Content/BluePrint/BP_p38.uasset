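; BP_p38 is a P-38 airplane actor that spins its two propellers and moves steadily forward through the level.
; Each tick it rolls the Left and Right components by PropellerRotateSpeed scaled by delta time, with the right one reversed to counter-rotate.
; It also offsets the whole actor along world X at a fixed frame-rate-independent speed, regardless of its facing.
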(event EventTick
  (params (DeltaSeconds :type Float%20%28single-precision%29))
  (Variables|Default|SetDelta%20Seconds DeltaSeconds) ; tick이벤트 델타세컨드 변수승격
  ;[1 1 1] 왼쪽 프로펠러 회전
  (Transformation|AddLocalRotation (Variables|Default|GetLeft) (Math|Rotator|MakeRotator (* (Variables|Default|GetPropeller%20Rotate%20Speed) (Utilities|Time|GetWorldDeltaSeconds)) 0.0 0.0) false false)
  ;[1 1 1] 오른쪽 프로펠러 회전
  (Transformation|AddLocalRotation (Variables|Default|GetRight) (Math|Rotator|MakeRotator (* (Variables|Default|GetDelta%20Seconds) (Variables|Default|GetPropeller%20Rotate%20Speed) -1.0) 0.0 0.0) false false)
  ;[1 1 1] 비행기 이동
  (Transformation|AddActorWorldOffset (Math|Vector|MakeVector (* (Utilities|Time|GetWorldDeltaSeconds) 6e+01) 0.0 0.0)))

(fn ConstructionScript)