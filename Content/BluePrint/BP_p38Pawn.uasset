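; Player-controllable P-38 airplane pawn that flies forward continuously at a fixed speed along its local X axis.
; Tick spins the left and right propellers in opposite directions using a shared speed variable and moves the actor forward.
; Pitch and Roll axis inputs rotate the whole actor in local space, so they steer the flight path.
; All movement and rotation scale by world delta seconds for frame-rate independence.
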(event EventTick
  (params (DeltaSeconds :type Float%20%28single-precision%29))
  (Variables|Default|SetDelta%20Seconds DeltaSeconds) ; tick이벤트 델타세컨드 변수승격
  ;[1 1 1] 왼쪽 프로펠러 회전
  (Transformation|AddLocalRotation (Variables|Default|GetLeft) (Math|Rotator|MakeRotator (* (Variables|Default|GetPropeller%20Rotate%20Speed) (Utilities|Time|GetWorldDeltaSeconds)) 0.0 0.0) false false)
  ;[1 1 1] 오른쪽 프로펠러 회전
  (Transformation|AddLocalRotation (Variables|Default|GetRight) (Math|Rotator|MakeRotator (* (Utilities|Time|GetWorldDeltaSeconds) (Variables|Default|GetPropeller%20Rotate%20Speed) -1.0) 0.0 0.0) false false)
  ;[1 1 1] 비행기 이동
  (Transformation|AddActorLocalOffset (Math|Vector|MakeVector (* (Utilities|Time|GetWorldDeltaSeconds) 6e+01) 0.0 0.0) false false))

(event Input|AxisEvents|InputAxisRoll
  (params (AxisValue :type Float%20%28single-precision%29))
  ;[1 1 1] Roll 회전
  (Transformation|AddActorLocalRotation (Math|Rotator|MakeRotator (* AxisValue 6e+01 (Utilities|Time|GetWorldDeltaSeconds)) 0.0 0.0) false false))

(event Input|AxisEvents|InputAxisPitch
  (params (AxisValue :type Float%20%28single-precision%29))
  ;[1 1 1] Pitch 회전
  (Transformation|AddActorLocalRotation (Math|Rotator|MakeRotator 0.0 (* AxisValue 6e+01 (Utilities|Time|GetWorldDeltaSeconds)) 0.0) false false))

(fn ConstructionScript)