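; BP_P381 is a player-controlled aircraft pawn that constantly flies forward with spinning propellers.
; Each tick it adds full movement input along its forward vector and rolls the Left and Right components in opposite directions at the 프러펠러회전 (propeller rotation) speed.
; Roll and Pitch axis inputs rotate the actor locally at a fixed rate, scaled by delta time, which steers the flight direction.
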(event EventTick
  (params (DeltaSeconds :type Float%20%28single-precision%29))
  (Utilities|FlowControl|Sequence
    (:then_0
      (Transformation|AddLocalRotation (Variables|Default|Getleft) (Math|Rotator|MakeRotator (* (Variables|속력|Get프러펠러%20회전) (Utilities|Time|GetWorldDeltaSeconds)) 0.0 0.0) false false))
    (:then_1
      (Pawn|Input|AddMovementInput (Transformation|GetActorForwardVector) 1.0 false))
    (:then_2
      (Transformation|AddLocalRotation (Variables|Default|Getright) (Math|Rotator|MakeRotator (* (Variables|속력|Get프러펠러%20회전) (Utilities|Time|GetWorldDeltaSeconds) -1.0) 0.0 0.0) false false))))

(event Input|AxisEvents|InputAxisRoll
  (params (AxisValue :type Float%20%28single-precision%29))
  (Transformation|AddActorLocalRotation (Math|Rotator|MakeRotator (* AxisValue 6e+01 (Utilities|Time|GetWorldDeltaSeconds)) 0.0 0.0) false false))

(event Input|AxisEvents|InputAxisPitch
  (params (AxisValue :type Float%20%28single-precision%29))
  (Transformation|AddActorLocalRotation (Math|Rotator|MakeRotator 0.0 (* AxisValue 6e+01 (Utilities|Time|GetWorldDeltaSeconds)) 0.0) false false))

(fn ConstructionScript)